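; Actor that simulates a 360-degree laser scanner and publishes its readings to ROS through a TempoROS node.
; Each tick it line-traces once per degree around world yaw from its location, with debug drawing.
; The hit distances are joined into a bracketed, comma-separated string and published on the "scan_sim" topic.
; It also sets a constant diagonal physics velocity on its Cube every tick, then clears the scan buffers.
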(event `self.ReceiveBeginPlay`
  (bind _returnvalue (`TempoROSNodeBlueprintFunctionLibrary.CreateTempoROSNode` "MyNode" false))
  (bind _output_get (set `self.ROSNode` _returnvalue))
  (`TempoROSTempoROSBlueprintFunctionLibrary.AddStringPublisher` _output_get "scan_sim" (struct :`bLimitedQueueSize` true :`Reliability` "SystemDefault" :`Durability` "SystemDefault" :`bCustomDeadline` true :`bCustomLifespan` true :`Liveliness` "SystemDefault")))

(event `self.ReceiveTick`
  (params (DeltaSeconds :type "Float (single-precision)"))
  (bind _returnvalue (`self.K2_GetActorLocation`))
  (bind _outputstring (`self.OutputString`))
  (for _index (range 360)
    (bind _outhit (`KismetSystemLibrary.LineTraceSingle` :`Start` _returnvalue :`End` (+ _returnvalue (* (`KismetMathLibrary.GetForwardVector` (`KismetMathLibrary.MakeRotator` 0.0 0.0 (* (`KismetMathLibrary.Conv_IntToDouble` _index) 1.0))) (1000.0 1000.0 1000.0))) :`TraceChannel` "TraceTypeQuery1" :`DrawDebugType` "ForOneFrame"))
    (`KismetArrayLibrary.Array_Add` (`self.RayDistances`) (`.Distance` (`GameplayStatics.BreakHitResult` _outhit))))
  (for _array_element (`self.RayDistances`)
    (`KismetArrayLibrary.Array_Add` _outputstring (`KismetStringLibrary.Conv_DoubleToString` _array_element)))
  (`TempoROSTempoROSBlueprintFunctionLibrary.PublishString` (`self.ROSNode`) "scan_sim" (`KismetStringLibrary.Concat_StrStr` (`KismetStringLibrary.Concat_StrStr` (`KismetStringLibrary.Concat_StrStr` (`self.out_string`) "[") (`KismetStringLibrary.JoinStringArray` _outputstring ",")) "]"))
  (`PrimitiveComponent.SetPhysicsLinearVelocity` (`self.Cube`) (100.0 100.0 0.0) false "None")
  (`KismetArrayLibrary.Array_Clear` (`self.RayDistances`))
  (`KismetArrayLibrary.Array_Clear` (`self.OutputString`))
  (set `self.out_string` ""))

(fn `UserConstructionScript`)