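; BP_ExAu is an actor that triggers effects and audio from keyboard presses, apparently for testing.
; Number keys 0, 2, 3 and 4 each call FXManager to play an explosion or fire effect at a hardcoded offset.
; K plays a background sound through RedAudioManager alongside a distant atomic bomb effect.
; BeginPlay, overlap, Tick and the construction script are empty.
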(event `Key|K`
  (params (Key :type "Key Structure"))
  (:`Pressed`
    (`RedAudioManagerComponent.PlaySound` (`self.RedAudioManager`) "Background_Confession" (0.0 0.0 0.0))
    (`FXManagerComponent.PlayFX` :`self` (`self.FXManager`) :`Type` "Atomic_Bomb" :`Offset` (0.0 9000.0 0.0))))

(event `Key|Two`
  (params (Key :type "Key Structure"))
  (:`Pressed`
    (`FXManagerComponent.PlayFX` :`self` (`self.FXManager`) :`Type` "Explosion_General_M_03" :`Offset` (200.0 200.0 0.0))))

(event `Key|Zero`
  (params (Key :type "Key Structure"))
  (:`Pressed`
    (`FXManagerComponent.PlayFX` :`self` (`self.FXManager`) :`Type` "Explosion_Car")))

(event `Key|Three`
  (params (Key :type "Key Structure"))
  (:`Pressed`
    (`FXManagerComponent.PlayFX` :`self` (`self.FXManager`) :`Type` "Explosion_General_Mass_03" :`Offset` (200.0 500.0 0.0))))

(event `Key|Four`
  (params (Key :type "Key Structure"))
  (:`Pressed`
    (`FXManagerComponent.PlayFX` :`self` (`self.FXManager`) :`Type` "Fire_01" :`Offset` (200.0 700.0 0.0))))

(fn `UserConstructionScript`)